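; RPG stat component that stores attributes, each with inherited stats keyed by gameplay tag, as base, bonus and current values.
; Modify functions write through clamped setters, and current-value subtraction targets bonus before base.
; Attribute changes scale their inherited stats, then Health, Mana and Exp checks handle death, max caps and Exp rollover into Level.
; Level gains award attribute points and call OnLevelUP; numpad debug keys adjust Strength.
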(event Custom|CheckExp
  (bind _returnvalue (Stats|Getters|GetStatValue "NewEnumerator3" "(TagName=\"Attribute.Exp\")"))
  (bind _returnvalue_2 (Stats|Getters|GetStatValue "NewEnumerator3" "(TagName=\"Attribute.MaxExp\")"))
  (if (>= _returnvalue _returnvalue_2)
    (Stats|Setters|SetStat "NewEnumerator1" "(TagName=\"Attribute.Exp\")" (- _returnvalue _returnvalue_2))
    (Attributes|Function|ModifyAttribute "NewEnumerator0" "NewEnumerator1" "(TagName=\"Attribute.Level\")" 1.0)))

(event Custom|CheckHealth
  (bind _returnvalue (Stats|Getters|GetStatValue "NewEnumerator3" "(TagName=\"Attribute.Health\")"))
  (if (<= _returnvalue 0.0)
    (Default|CallOnDeath)
    (elif (> _returnvalue (Stats|Getters|GetStatValue "NewEnumerator3" "(TagName=\"Attribute.HealthMax\")"))
      (Stats|Setters|SetStat "NewEnumerator1" "(TagName=\"Attribute.Health\")" (Stats|Getters|GetStatValue "NewEnumerator1" "(TagName=\"Attribute.HealthMax\")"))
      (Stats|Setters|SetStat "NewEnumerator2" "(TagName=\"Attribute.Health\")" (Stats|Getters|GetStatValue "NewEnumerator2" "(TagName=\"Attribute.HealthMax\")")))))

(event Custom|CheckMana
  (if (> (Stats|Getters|GetStatValue "NewEnumerator3" "(TagName=\"Attribute.Mana\")") (Stats|Getters|GetStatValue "NewEnumerator3" "(TagName=\"Attribute.ManaMax\")"))
    (Stats|Setters|SetStat "NewEnumerator1" "(TagName=\"Attribute.Mana\")" (Stats|Getters|GetStatValue "NewEnumerator1" "(TagName=\"Attribute.ManaMax\")"))
    (Stats|Setters|SetStat "NewEnumerator2" "(TagName=\"Attribute.Mana\")" (Stats|Getters|GetStatValue "NewEnumerator2" "(TagName=\"Attribute.ManaMax\")"))))

(event EventBeginPlay)

(event Input|KeyboardEvents|DebugKeyNumPadTwo
  (params (Key :type Key%20Structure) (ActionValue :type Input%20Action%20Value%20Structure))
  (:Pressed
    (Attributes|Function|ModifyAttribute "NewEnumerator1" "NewEnumerator1" "(TagName=\"Attribute.Strength\")" 1.0)))

(event Input|KeyboardEvents|DebugKeyNumPadOne
  (params (Key :type Key%20Structure) (ActionValue :type Input%20Action%20Value%20Structure))
  (:Pressed
    (Attributes|Function|ModifyAttribute "NewEnumerator0" "NewEnumerator1" "(TagName=\"Attribute.Strength\")" 1.0)))

(fn GetAttributeRef
  (params (Attribute :type Gameplay%20Tag%20Structure))
  (for (_array_element _array_index) (Utilities|Struct|BreakF_PlayerAttribute (Variables|Default|GetAttributes))
    (LocalVariables|SetL_AttributeValue _array_element)
    (LocalVariables|SetL_AttributeIndex _array_index)
    (if (== Attribute (.Name (Utilities|Struct|BreakF_SingleAttribute _array_element)))
      (return (LocalVariables|GetL_AttributeValue) (LocalVariables|GetL_AttributeIndex)))))

(fn GetStatRef
  (params (Stat :type Gameplay%20Tag%20Structure))
  (for (_array_element _array_index) (Utilities|Struct|BreakF_PlayerAttribute (Variables|Default|GetAttributes))
    (bind _output_get (LocalVariables|SetL_Attribute _array_element))
    (LocalVariables|SetL_AttributeIndex _array_index)
    (for (_array_element_2 _array_index_2) (.StatsInherited (Utilities|Struct|BreakF_SingleAttribute _output_get))
      (LocalVariables|SetL_StatAttribute _array_element_2)
      (LocalVariables|SetL_StatIndex _array_index_2)
      (if (== Stat (Utilities|Struct|BreakF_Attribute _array_element_2))
        (return (LocalVariables|GetL_Attribute) (LocalVariables|GetL_AttributeIndex) (LocalVariables|GetL_StatAttribute) (LocalVariables|GetL_StatIndex))))))

(fn GetAttributeValue
  (params (Type :type E_Stat_Type%20Enum :default "NewEnumerator0") (Attribute :type Gameplay%20Tag%20Structure))
  (bind _returnattribute (Attributes|Getters|GetAttributeRef Attribute))
  (bind (_basevaluedefault _currentvaluetotal _multipliervaluebonus) (Utilities|Struct|BreakF_SingleAttribute _returnattribute))
  (return (Utilities|Select :Index Type :NewEnumerator0 -1.0 :NewEnumerator1 _basevaluedefault :NewEnumerator3 _multipliervaluebonus :NewEnumerator2 _currentvaluetotal)))

(fn ModifyAttribute
  (params (Operation :type E_Operations%20Enum :default "NewEnumerator0") (Type :type E_Stat_Type%20Enum :default "NewEnumerator0") (Attribute :type Gameplay%20Tag%20Structure) (Value :type Float%20%28double-precision%29))
  (bind _returnvalue (Attributes|Getters|GetAttributeValue Type Attribute))
  (switch Utilities|FlowControl|Switch|SwitchonE_Stat_Type Type
    (:NewEnumerator0
      (Development|PrintString "Warning: Modify Attribute - 
Error: Attribute is set to \"None\"")
      (return))
    (:NewEnumerator1
      _)
    (:NewEnumerator3
      _)
    (:NewEnumerator2
      (Attributes|Function|OperateCurrentValueAttribute Operation Attribute Value)
      (return)))
  (LocalVariables|SetL_AttributeFloat _returnvalue)
  (LocalVariables|SetL_CalculationFloat (Utilities|Select :Index Operation :NewEnumerator0 (+ _returnvalue Value) :NewEnumerator1 (- _returnvalue Value) :NewEnumerator2 Value))
  (Attributes|Setters|SetAttribute Type Attribute (LocalVariables|GetL_CalculationFloat))
  (Attributes|Function|ScalingStat Type Operation (.ReturnAttribute (Attributes|Getters|GetAttributeRef Attribute)) (Math|Float|SelectFloat Value (LocalVariables|GetL_AttributeFloat) (> (LocalVariables|GetL_CalculationFloat) 0.0)))
  (if (and (== Attribute "(TagName=\"Attribute.Level\")") (Utilities|Enum|Equal(Enum) Operation "NewEnumerator0"))
    (CallFunction|LevelUp Value)))

(fn SetAttribute
  (params (Type :type E_Stat_Type%20Enum :default "NewEnumerator0") (Attribute :type Gameplay%20Tag%20Structure) (Value :type Float%20%28double-precision%29))
  (bind (_returnattribute _returnattributeindex) (Attributes|Getters|GetAttributeRef Attribute))
  (bind _max (Variables|Default|GetMax))
  (bind _max_2 (Variables|Default|GetMax))
  (LocalVariables|SetL_SetAttribute _returnattribute)
  (LocalVariables|SetL_SetAttributeIndex _returnattributeindex)
  (switch Utilities|FlowControl|Switch|SwitchonE_Stat_Type Type
    (:NewEnumerator1
      (Utilities|Struct|SetmembersinF_SingleAttribute (LocalVariables|GetL_SetAttribute) (Math|Float|Clamp(Float) Value 0.0 _max_2) (Math|Float|Clamp(Float) (+ Value (Utilities|Struct|BreakF_SingleAttribute (LocalVariables|GetL_SetAttribute))) (Utilities|Struct|BreakF_SingleAttribute (LocalVariables|GetL_SetAttribute)) _max_2)))
    (:NewEnumerator3
      (Utilities|Struct|SetmembersinF_SingleAttribute (LocalVariables|GetL_SetAttribute) (Math|Float|Clamp(Float) (+ Value (Utilities|Struct|BreakF_SingleAttribute (LocalVariables|GetL_SetAttribute))) (Utilities|Struct|BreakF_SingleAttribute (LocalVariables|GetL_SetAttribute)) _max) (Math|Float|Clamp(Float) Value 0.0 _max)))
    (:NewEnumerator2
      (Development|PrintString "Warning: Set Attribute - 
Error: Can not use \"Current\"")
      (return)))
  (Utilities|Array|SetArrayElem (Utilities|Struct|BreakF_PlayerAttribute (Variables|Default|GetAttributes)) (LocalVariables|GetL_SetAttributeIndex) (LocalVariables|GetL_SetAttribute))
  (return))

(fn SetStat
  (params (Type :type E_Stat_Type%20Enum :default "NewEnumerator0") (Stat :type Gameplay%20Tag%20Structure) (Value :type Float%20%28double-precision%29))
  (bind _max (Variables|Default|GetMax))
  (bind _max_2 (Variables|Default|GetMax))
  (LocalVariables|SetL_Stat (.ReturnStat (Stats|Getters|GetStatRef Stat)))
  (switch Utilities|FlowControl|Switch|SwitchonE_Stat_Type Type
    (:NewEnumerator1
      (Utilities|Struct|SetmembersinF_Attribute (LocalVariables|GetL_Stat) (Math|Float|Clamp(Float) Value 0.0 _max) (Math|Float|Clamp(Float) (+ Value (Utilities|Struct|BreakF_Attribute (LocalVariables|GetL_Stat))) (Utilities|Struct|BreakF_Attribute (LocalVariables|GetL_Stat)) _max)))
    (:NewEnumerator3
      (Utilities|Struct|SetmembersinF_Attribute (LocalVariables|GetL_Stat) (Math|Float|Clamp(Float) (+ Value (Utilities|Struct|BreakF_Attribute (LocalVariables|GetL_Stat))) (Utilities|Struct|BreakF_Attribute (LocalVariables|GetL_Stat)) _max_2) (Math|Float|Clamp(Float) Value _max_2)))
    (:NewEnumerator2
      (Development|PrintString "Warning: Set Stat - 
Error: Can not use \"CurrentValue\"")
      (return)))
  (Stats|Setters|SetStatMember Stat (LocalVariables|GetL_Stat))
  (return))

(fn OperateCurrentValueAttribute
  (params (Operation :type E_Operations%20Enum :default "NewEnumerator0") (Attribute :type Gameplay%20Tag%20Structure) (Value :type Float%20%28double-precision%29))
  (switch Utilities|FlowControl|Switch|SwitchonE_Operations Operation
    (:NewEnumerator0
      (Attributes|Function|ModifyAttribute "NewEnumerator0" "NewEnumerator1" Attribute Value))
    (:NewEnumerator1
      (if (>= (- (Attributes|Getters|GetAttributeValue "NewEnumerator3" Attribute) Value) 0.0)
        (Attributes|Function|ModifyAttribute "NewEnumerator1" "NewEnumerator3" Attribute Value)
        (else
          (bind _output_get (LocalVariables|SetL_StoredValue (Attributes|Getters|GetAttributeValue "NewEnumerator3" Attribute)))
          (Attributes|Function|ModifyAttribute "NewEnumerator1" "NewEnumerator3" Attribute _output_get)
          (Attributes|Function|ModifyAttribute "NewEnumerator1" "NewEnumerator1" Attribute (- Value (LocalVariables|GetL_StoredValue))))))
    (:NewEnumerator2
      (Development|PrintString "Warning: Operate Current Value Attribute - 
Error:  Unable to Set \"Current\" Value")
      (return))))

(fn GetStatValue
  (params (Type :type E_Stat_Type%20Enum :default "NewEnumerator0") (Stat :type Gameplay%20Tag%20Structure))
  (bind _returnstat (Stats|Getters|GetStatRef Stat))
  (bind (_basevalue _currentvalue _multipliervalue) (Utilities|Struct|BreakF_Attribute _returnstat))
  (return (Utilities|Select :Index Type :NewEnumerator0 -1.0 :NewEnumerator1 _basevalue :NewEnumerator3 _multipliervalue :NewEnumerator2 _currentvalue)))

(fn ModifyStat
  (params (Operation :type E_Operations%20Enum :default "NewEnumerator0") (Type :type E_Stat_Type%20Enum :default "NewEnumerator0") (Stat :type Gameplay%20Tag%20Structure) (Value :type Float%20%28double-precision%29))
  (bind _returnvalue (Stats|Getters|GetStatValue Type Stat))
  (switch Utilities|FlowControl|Switch|SwitchonE_Stat_Type Type
    (:NewEnumerator0
      (Development|PrintString "Warning: Modify Stat - 
Error: Stat is set to \"None\"")
      (return))
    (:NewEnumerator1
      _)
    (:NewEnumerator3
      _)
    (:NewEnumerator2
      (Stats|Fuction|OperateCurrentValueStat Operation Stat Value)
      (return)))
  (Stats|Setters|SetStat Type Stat (Utilities|Select :Index Operation :NewEnumerator0 (+ _returnvalue Value) :NewEnumerator1 (- _returnvalue Value) :NewEnumerator2 Value))
  (Stats|Fuction|ConditionalStats Stat))

(fn SetStatMember
  (params (Stat :type Gameplay%20Tag%20Structure) (SingleStat :type F%20Attribute%20Structure))
  (bind (_returnattribute _returnattributeindex _returnstat _returnstatindex) (Stats|Getters|GetStatRef Stat))
  (bind _attributes (Variables|Default|GetAttributes))
  (bind _attributes_2 (Utilities|Struct|BreakF_PlayerAttribute _attributes))
  (LocalVariables|SetL_ReturnAttributeIndex _returnattributeindex)
  (bind _output_get (LocalVariables|SetL_StatArray (Utilities|Struct|BreakF_SingleAttribute _returnattribute)))
  (Utilities|Array|SetArrayElem _output_get _returnstatindex SingleStat)
  (bind _structout (Utilities|Struct|SetmembersinF_SingleAttribute (Utilities|Array|Get(acopy) _attributes_2 (LocalVariables|GetL_ReturnAttributeIndex)) (LocalVariables|GetL_StatArray)))
  (Utilities|Array|SetArrayElem _attributes_2 (LocalVariables|GetL_ReturnAttributeIndex) _structout)
  (return))

(fn OperateCurrentValueStat
  (params (Operations :type E_Operations%20Enum :default "NewEnumerator0") (Stat :type Gameplay%20Tag%20Structure) (Value :type Float%20%28double-precision%29))
  (switch Utilities|FlowControl|Switch|SwitchonE_Operations Operations
    (:NewEnumerator0
      (Stats|Fuction|ModifyStat "NewEnumerator0" "NewEnumerator1" Stat Value))
    (:NewEnumerator1
      (if (>= (- (Stats|Getters|GetStatValue "NewEnumerator3" Stat) Value) 0.0)
        (Stats|Fuction|ModifyStat "NewEnumerator1" "NewEnumerator3" Stat Value)
        (else
          (LocalVariables|SetL_StoredValue (Stats|Getters|GetStatValue "NewEnumerator3" Stat))
          (Stats|Fuction|ModifyStat "NewEnumerator1" "NewEnumerator3" Stat Value)
          (Stats|Fuction|ModifyStat "NewEnumerator1" "NewEnumerator1" Stat (- Value (LocalVariables|GetL_StoredValue))))))
    (:NewEnumerator2
      (Development|PrintString "Warning: Operate CurrentValue Stat - 
Error:  Unable to Set \"Current\" Value"))))

(fn ScalingStat
  (params (Type :type E_Stat_Type%20Enum :default "NewEnumerator0") (Operation :type E_Operations%20Enum :default "NewEnumerator0") (Attribute :type F%20Single%20Attribute%20Structure) (Value :type Float%20%28double-precision%29))
  (for _array_element (Utilities|Struct|BreakF_SingleAttribute Attribute)
    (LocalVariables|SetLocalStat (.AttributeTag (Utilities|Struct|BreakF_Attribute _array_element)))
    (Stats|Setters|SetStat Type (LocalVariables|GetLocalStat) (Math|Float|Clamp(Float) (Utilities|Select :Index Operation :NewEnumerator0 (+ (Utilities|Select :Index Type :NewEnumerator0 -1.0 :NewEnumerator1 (.BaseValue (Utilities|Struct|BreakF_Attribute _array_element)) :NewEnumerator3 (.MultiplierValue (Utilities|Struct|BreakF_Attribute _array_element)) :NewEnumerator2 0.0) (* (.MultiplierValue (Utilities|Struct|BreakF_Attribute _array_element)) Value)) :NewEnumerator1 (- (Utilities|Select :Index Type :NewEnumerator0 -1.0 :NewEnumerator1 (.BaseValue (Utilities|Struct|BreakF_Attribute _array_element)) :NewEnumerator3 (.MultiplierValue (Utilities|Struct|BreakF_Attribute _array_element)) :NewEnumerator2 0.0) (* (.MultiplierValue (Utilities|Struct|BreakF_Attribute _array_element)) Value)) :NewEnumerator2 (* (.MultiplierValue (Utilities|Struct|BreakF_Attribute _array_element)) Value)) 0.0 (Variables|Default|GetMax)))
    (Stats|Fuction|ConditionalStats (LocalVariables|GetLocalStat))))

(fn ConditionalStats
  (params (Stat :type Gameplay%20Tag%20Structure))
  (|SwitchGameplayTag Stat
    (:Attribute.Exp
      (CallFunction|CheckExp))
    (:Attribute.Health
      (CallFunction|CheckHealth))
    (:Attribute.Mana
      (CallFunction|CheckMana))))

(fn LevelUp
  (params (Value :type Float%20%28double-precision%29))
  (Attributes|Function|ModifyAttribute "NewEnumerator0" "NewEnumerator1" "(TagName=\"Attribute.AttributePoints\")" (* Value 3.0))
  (Default|CallOnLevelUP))

(fn Initialize
  (params (Attributes :type F%20Player%20Attribute%20Structure))
  (Variables|Default|SetAttributes Attributes))