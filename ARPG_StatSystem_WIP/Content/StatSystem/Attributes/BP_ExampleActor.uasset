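; Example actor for the attribute stat system that initializes its BPAttributesComponent on BeginPlay and then reads an attribute value.
; GetAttribtueValue queries an attribute component for the current value of the first attribute tag in PlayerInfoRef, though BeginPlay passes it no component.
; Nodes for setting a base value and building an FAttribute are left disconnected, so the read value has no effect.
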(event `self.ReceiveBeginPlay`
  (`/Game/AdvancedARPGCombat/AdvancedCombatFramework/AttributesSystem/BP_AttributesComponent.Initialize` (`self.BP_AttributesComponent`))
  (bind _attributevalue (`self.GetAttribtueValue` null)))

(fn `GetAttribtueValue`
  (params (AttributeComponent :type "/Game/AdvancedARPGCombat/AdvancedCombatFramework/AttributesSystem/BP_AttributesComponent Object Reference"))
  (returns (AttributeValue :type "Float (double-precision)"))
  (bind _output_get (set `self.AttribueValue` (`/Game/AdvancedARPGCombat/AdvancedCombatFramework/AttributesSystem/BP_AttributesComponent.Get Current Attribute Value` AttributeComponent (`.AttributeTag_27_175E28554750400542EF3F8A57A404B9` (break `/Game/AdvancedARPGCombat/AdvancedCombatFramework/AttributesSystem/Structs/F_Attribute` (`|GetArrayItem` (`/Game/AdvancedARPGCombat/AdvancedCombatFramework/CoreCombatSystem/DataAssets/BP_PlayerInfo.Attributes` (`self.PlayerInfoRef`))))))))
  (return _output_get))

(fn `UserConstructionScript`)